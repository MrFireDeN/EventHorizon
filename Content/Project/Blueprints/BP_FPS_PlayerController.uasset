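; First-person shooter player controller that turns player input into actions on its BP_FPS_Character.
; It caches the character on BeginPlay, where non-dedicated instances also draw the character HUD, and on possession through SetPlayer.
; Input drives movement, look, jump, sprint speed, current-gun firing and aim zoom, which divides default FOV by the gun's AimScale.
; Hardcoded number keys swap between rifle, shotgun, SMG, sniper and pistol classes.
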(event Custom|SetPlayer
  (params (Player :type Pawn%20Object%20Reference))
  (bind _asbp_fps_character (Utilities|Casting|CastToBP_FPS_Character Player))
  (Variables|Default|SetAs%20BP%20FPS%20Character _asbp_fps_character)
  (Input|EnableInput self))

(event EventBeginPlay
  (if (not (Networking|IsDedicatedServer))
    (bind _asbp_fps_character (Utilities|Casting|CastToBP_FPS_Character (Pawn|GetControlledPawn))
      (:then
        (Variables|Default|SetAs%20BP%20FPS%20Character _asbp_fps_character)
        (bind _asbp_fps_hud (Utilities|Casting|CastToBP_FPS_HUD (HUD|GetHUD)))
        (bind _output_get (Variables|Default|SetAs%20BP%20FPS%20HUD _asbp_fps_hud))
        (Default|DrawCharacterHUD _output_get))
      (:CastFailed
        (Development|PrintString "NO FPS CHARACTER IN PLAYER CONTROLLER" true true "(R=1.000000,G=0.000000,B=0.000000,A=1.000000)" 2.0 "Error")))))

(event EventTick
  (params (DeltaSeconds :type Float%20%28single-precision%29)))

(event EventPossess
  (params (PossessedPawn :type Pawn%20Object%20Reference))
  (CallFunction|SetPlayer PossessedPawn))

(event Input|ActionEvents|InputActionJump
  (params (Key :type Key%20Structure :default "None"))
  (bind _as_bp_fps_character (Variables|Default|GetAs%20BP%20FPS%20Character))
  (bind _as_bp_fps_character_2 (Variables|Default|GetAs%20BP%20FPS%20Character))
  ;[0.651 0.2359 0 0.5] Movement
  (:Pressed
    (Utilities|IsValid _as_bp_fps_character
      (:Is%20Valid
        (Character|Jump _as_bp_fps_character_2))))
  (:Released
    (Utilities|IsValid _as_bp_fps_character
      (:Is%20Valid
        (Character|StopJumping _as_bp_fps_character_2)))))

(event Input|ActionEvents|InputActionSprint
  (params (Key :type Key%20Structure :default "None"))
  (bind _as_bp_fps_character (Variables|Default|GetAs%20BP%20FPS%20Character))
  (bind _as_bp_fps_character_2 (Variables|Default|GetAs%20BP%20FPS%20Character))
  (bind _charactermovement (Variables|/Script/Engine.Character|GetCharacterMovement _as_bp_fps_character_2))
  ;[0.651 0.2359 0 0.5] Movement
  (:Pressed
    (Utilities|IsValid _as_bp_fps_character
      (:Is%20Valid
        (Variables|/Script/Engine.CharacterMovementComponent|SetMaxWalkSpeed _charactermovement (Variables|/Game/Project/Blueprints/BP_FPS_Character.BP_FPS_Character_C|GetRunSpeed _as_bp_fps_character_2)))))
  (:Released
    (Utilities|IsValid _as_bp_fps_character
      (:Is%20Valid
        (Variables|/Script/Engine.CharacterMovementComponent|SetMaxWalkSpeed _charactermovement (Variables|/Game/Project/Blueprints/BP_FPS_Character.BP_FPS_Character_C|GetWalkSpeed _as_bp_fps_character_2))))))

(event Input|ActionEvents|InputActionFire
  (params (Key :type Key%20Structure :default "None"))
  (bind _as_bp_fps_character (Variables|Default|GetAs%20BP%20FPS%20Character))
  (bind _currentgun (Variables|/Game/Project/Blueprints/BP_FPS_Character.BP_FPS_Character_C|GetCurrentGun _as_bp_fps_character))
  (:Pressed
    (Default|StartFire _currentgun))
  (:Released
    (Default|StopFire _currentgun)))

(event Input|ActionEvents|InputActionAim
  (params (Key :type Key%20Structure :default "None"))
  (bind _as_bp_fps_character (Variables|Default|GetAs%20BP%20FPS%20Character))
  (bind _as_bp_fps_character_2 (Variables|Default|GetAs%20BP%20FPS%20Character))
  (bind _camera (Variables|/Game/Project/Blueprints/BP_FPS_Character.BP_FPS_Character_C|GetCamera _as_bp_fps_character))
  (:Pressed
    (Utilities|IsValid _as_bp_fps_character_2
      (:Is%20Valid
        (Camera|SetFieldOfView _camera (/ (Variables|Default|GetDefaultFOV) (Variables|/Game/Project/Blueprints/BP_Gun_BASE.BP_Gun_BASE_C|GetAimScale (Variables|/Game/Project/Blueprints/BP_FPS_Character.BP_FPS_Character_C|GetCurrentGun (Variables|Default|GetAs%20BP%20FPS%20Character))))))))
  (:Released
    (Utilities|IsValid _as_bp_fps_character_2
      (:Is%20Valid
        (Camera|SetFieldOfView _camera (Variables|Default|GetDefaultFOV))))))

(event Input|AxisEvents|InputAxisMoveForward
  (params (AxisValue :type Float%20%28single-precision%29))
  (bind _as_bp_fps_character (Variables|Default|GetAs%20BP%20FPS%20Character))
  ;[0.651 0.2359 0 0.5] Movement
  (Utilities|IsValid _as_bp_fps_character
    (:Is%20Valid
      (Pawn|Input|AddMovementInput _as_bp_fps_character (Transformation|GetActorForwardVector _as_bp_fps_character) AxisValue false))))

(event Input|AxisEvents|InputAxisMoveRight
  (params (AxisValue :type Float%20%28single-precision%29))
  (bind _as_bp_fps_character (Variables|Default|GetAs%20BP%20FPS%20Character))
  ;[0.651 0.2359 0 0.5] Movement
  (Utilities|IsValid _as_bp_fps_character
    (:Is%20Valid
      (Pawn|Input|AddMovementInput _as_bp_fps_character (Transformation|GetActorRightVector _as_bp_fps_character) AxisValue false))))

(event Input|AxisEvents|InputAxisLookUp
  (params (AxisValue :type Float%20%28single-precision%29))
  (bind _as_bp_fps_character (Variables|Default|GetAs%20BP%20FPS%20Character))
  ;[0.651 0.2359 0 0.5] Movement
  (Utilities|IsValid _as_bp_fps_character
    (:Is%20Valid
      (Pawn|Input|AddControllerPitchInput _as_bp_fps_character AxisValue))))

(event Input|AxisEvents|InputAxisLookRight
  (params (AxisValue :type Float%20%28single-precision%29))
  (bind _as_bp_fps_character (Variables|Default|GetAs%20BP%20FPS%20Character))
  ;[0.651 0.2359 0 0.5] Movement
  (Utilities|IsValid _as_bp_fps_character
    (:Is%20Valid
      (Pawn|Input|AddControllerYawInput _as_bp_fps_character AxisValue))))

(event Input|KeyboardEvents|5
  (params (Key :type Key%20Structure :default "None"))
  (bind _as_bp_fps_character (Variables|Default|GetAs%20BP%20FPS%20Character))
  ;[0.15 0.15 0.15 0.5] Change Gun
  (:Pressed
    (Utilities|IsValid _as_bp_fps_character
      (:Is%20Valid
        (Default|ChangeGun _as_bp_fps_character "/Game/Project/Blueprints/Guns/BP_Pistol_BASE_Child.BP_Pistol_BASE_Child_C")))))

(event Input|KeyboardEvents|1
  (params (Key :type Key%20Structure :default "None"))
  (bind _as_bp_fps_character (Variables|Default|GetAs%20BP%20FPS%20Character))
  ;[0.15 0.15 0.15 0.5] Change Gun
  (:Pressed
    (Utilities|IsValid _as_bp_fps_character
      (:Is%20Valid
        (Default|ChangeGun _as_bp_fps_character "/Game/Project/Blueprints/Guns/BP_AssultRifle_BASE.BP_AssultRifle_BASE_C")))))

(event Input|KeyboardEvents|2
  (params (Key :type Key%20Structure :default "None"))
  (bind _as_bp_fps_character (Variables|Default|GetAs%20BP%20FPS%20Character))
  ;[0.15 0.15 0.15 0.5] Change Gun
  (:Pressed
    (Utilities|IsValid _as_bp_fps_character
      (:Is%20Valid
        (Default|ChangeGun _as_bp_fps_character "/Game/Project/Blueprints/Guns/BP_Shotgun_BASE.BP_Shotgun_BASE_C")))))

(event Input|KeyboardEvents|3
  (params (Key :type Key%20Structure :default "None"))
  (bind _as_bp_fps_character (Variables|Default|GetAs%20BP%20FPS%20Character))
  ;[0.15 0.15 0.15 0.5] Change Gun
  (:Pressed
    (Utilities|IsValid _as_bp_fps_character
      (:Is%20Valid
        (Default|ChangeGun _as_bp_fps_character "/Game/Project/Blueprints/Guns/BP_SMG_BASE.BP_SMG_BASE_C")))))

(event Input|KeyboardEvents|4
  (params (Key :type Key%20Structure :default "None"))
  (bind _as_bp_fps_character (Variables|Default|GetAs%20BP%20FPS%20Character))
  ;[0.15 0.15 0.15 0.5] Change Gun
  (:Pressed
    (Utilities|IsValid _as_bp_fps_character
      (:Is%20Valid
        (Default|ChangeGun _as_bp_fps_character "/Game/Project/Blueprints/Guns/BP_SniperRifle_BASE.BP_SniperRifle_BASE_C")))))

(fn ConstructionScript)