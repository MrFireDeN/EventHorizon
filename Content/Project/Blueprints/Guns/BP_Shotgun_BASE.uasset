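; BP_Shotgun_BASE is a shotgun Blueprint that supplies the multi-pellet hit trace for firing.
; TraceShoot casts one Visibility line trace per pellet (GrapesCount) from the shot source, ignoring the owning character.
; Each ray's forward direction gets random up and right offsets scaled by GrapesRadius, giving a square rather than circular spread.
; It returns every trace result as a hit array, including misses; the event graph is inactive.
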(event EventBeginPlay
  (|CallParentFunction) ; This node is disabled and will not be called.\nDrag off pins to build functionality.
)

(event Collision|EventActorBeginOverlap
  (params (OtherActor :type Actor%20Object%20Reference)))

(event EventTick
  (params (DeltaSeconds :type Float%20%28single-precision%29))
  (|CallParentFunction DeltaSeconds) ; This node is disabled and will not be called.\nDrag off pins to build functionality.
)

(fn ConstructionScript
  (|CallParentFunction))

(fn TraceShoot
  (params (ShotSource :type Scene%20Component%20Object%20Reference))
  (LocalVariables|SetShotStartPoint ShotSource)
  (Utilities|Array|Clear (Variables|Grapes|GetHitArray))
  (for _index (range 1 (Variables|Grapes|GetGrapesCount))
    (bind _outhit (Collision|LineTraceByChannel (Transformation|GetWorldLocation (LocalVariables|GetShotStartPoint)) (+ (Transformation|GetWorldLocation (LocalVariables|GetShotStartPoint)) (* (+ (Math|Vector|GetForwardVector (LocalVariables|GetShotStartPoint)) (* (Math|Vector|GetUpVector (LocalVariables|GetShotStartPoint)) (* (Variables|Grapes|GetGrapesRadius) (Math|Random|RandomFloatinRange -1.0 1.0))) (* (Math|Vector|GetRightVector (LocalVariables|GetShotStartPoint)) (* (Variables|Grapes|GetGrapesRadius) (Math|Random|RandomFloatinRange -1.0 1.0)))) 5000)) "TraceTypeQuery1" false (Utilities|Array|MakeArray (Variables|Default|GetCharacterOwner)) "None"))
    (Utilities|Array|Add (Variables|Grapes|GetHitArray) _outhit))
  (return (Variables|Grapes|GetHitArray)))