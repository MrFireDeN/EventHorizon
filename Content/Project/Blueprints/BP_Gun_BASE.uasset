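; Base networked hitscan gun that fires automatic or semi-automatic shots, with heat replacing ammo.
; A client camera trace that hits a "Damageable" actor triggers a server re-trace that applies point damage, alongside effects and interpolated recoil.
; Heat builds per shot and cools on Tick; reaching maximum blocks firing.
; One fire press while overheated acts as an active reload: inside the heat window it clears heat, otherwise it switches to fault cooling.
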(event Custom|StartFire
  ;[0.15 0 0 0.5] Start Fire Server
  (if (Variables|Reload|GetOverheated)
    ;;[0 1 0.08873 0.5] Cooling
    (Utilities|FlowControl|DoOnce false :!label _label
      (:Completed
        (if (Math|Float|InRange(Float) (Variables|Reload|GetHeat) (Variables|Reload|GetOverheatReloadPointMin) (Variables|Reload|GetOverheatReloadPointMax))
          (Variables|Reload|SetHeat 0.0)
          (Variables|Reload|SetOverheated false)
          (else
            (Variables|Reload|SetCoolingFault true)))))
    (else
      (Utilities|FlowControl|Sequence
        (:then_0
          (goto _label Reset))
        (:then_1
          (if (Variables|Global|GetCanFire)
            (CallFunction|TracefromClient)
            (CallFunction|ApplyFireEffects)
            (CallFunction|ApplyRecoil)
            (CallFunction|HeatUp)
            (CallFunction|PostShoot)))))))

(event Custom|SetSemiAutomaticTimer
  ;[0.15 0 0 0.5] Stop Fire Server
  (if (Variables|Global|GetShoted)
    (Variables|Global|SetShoted false)
    (if (> (Variables|Global|GetFirerate) 0.0)
      (Variables|Global|SetCanFire false)
      (Utilities|Time|SetTimerbyFunctionName 0 "SetCanFire" (Variables|Global|GetFirerate) false true))))

(event Custom|HeatRecovery
  (params (DeltaTime :type Float%20%28double-precision%29))
  ;[0 0.15 0.005085 0.5] Recovery
  ;;[0.15 0 0.004793 0.5] Heat Recovery Server
  (if (> (Variables|Reload|GetHeat) 0.0)
    (bind _output_get (Variables|Reload|SetHeat (Math|Float|Clamp(Float) (- (Variables|Reload|GetHeat) (* DeltaTime (select (Variables|Reload|GetCoolingFault) (Variables|Reload|GetCoolingMultiplierFault) (Variables|Reload|GetCoolingMultiplier)))) 0.0 (Variables|Reload|GetMaxHeat))))
    (if (== _output_get 0.0)
      (Variables|Reload|SetOverheated false)
      (Variables|Reload|SetCoolingFault false))))

(event Custom|SetCharacterOwner
  (params (Character :type BP%20FPS%20Character%20Object%20Reference))
  (Variables|Default|SetCharacterOwner Character))

(event Custom|TraceFromClient
  ;[0 0.03689 0.15 0.502] Trace From Client
  (bind _outhit (CallFunction|TraceShoot (Variables|/Game/Project/Blueprints/BP_FPS_Character.BP_FPS_Character_C|GetCamera (Variables|Default|GetCharacterOwner))))
  (bind _array_element (Utilities|Array|ForEachLoopwithBreak _outhit :!label _label)
    (:LoopBody
      (if (Utilities|IsValid (.HitActor (Collision|BreakHitResult _array_element)))
        (if (Actor|ActorHasTag (.HitActor (Collision|BreakHitResult _array_element)) "Damageable")
          (CallFunction|TracefromServer)
          (goto _label Break))))))

(event Custom|StopFire
  ;[0.15 0 0 0.5] Stop Fire Server
  (if (Variables|Global|GetAutomatic)
    (CallFunction|ClearStartFireTimer)
    (else
      (CallFunction|SetSemiAutomaticTimer))))

(event Custom|ApplyRecoil
  ;[0 0.535 0.8125 0.5] Recoil on Owning Client
  (Pawn|Input|AddControllerPitchInput (Variables|Default|GetCharacterOwner) (* (Variables|Global|GetRecoil) (Math|Random|RandomFloatinRange -1.0 -0.5)))
  (Pawn|Input|AddControllerYawInput (Variables|Default|GetCharacterOwner) (* (Variables|Global|GetRecoil) (Math|Random|RandomFloatinRange -0.25 0.25)))
  (Transformation|SetRelativeLocation (Variables|Default|GetMesh) "-10.000000,0.000000,0.000000" false false))

(event Custom|RecoilRecovery
  (params (DeltaTime :type Float%20%28single-precision%29))
  (bind _firerate (Variables|Global|GetFirerate))
  (bind _mesh (Variables|Default|GetMesh))
  (bind _relativelocation (Variables|/Script/Engine.SceneComponent|GetRelativeLocation _mesh))
  ;[0 0.15 0.005085 0.5] Recovery
  ;;[0.15 0.1277 0 0.5] Recoil Recovery on Owning Client
  (if (Utilities|Operators|NotEqual(!=) :A _relativelocation :ErrorTolerance 0.01)
    (Transformation|SetRelativeLocation (Variables|Default|GetMesh) (Math|Interpolation|VInterpTo _relativelocation "0, 0, 0" DeltaTime (select (> _firerate 0.0) (/ 1.0 _firerate) 1e+01)) false false)))

(event Custom|TraceFromServer
  ;[0 0.03689 0.15 0.502] Trace From Server
  (bind _outhit (CallFunction|TraceShoot (Variables|/Game/Project/Blueprints/BP_FPS_Character.BP_FPS_Character_C|GetCamera (Variables|Default|GetCharacterOwner))))
  (for _array_element _outhit
    (Game|Damage|ApplyPointDamage (.HitActor (Collision|BreakHitResult _array_element)) (Variables|Global|GetDamage) (.TraceStart (Collision|BreakHitResult _array_element)) _array_element (Pawn|GetController (Variables|Default|GetCharacterOwner)) self)))

(event Custom|ApplyFireEffects
  ;[0.15 0 0.1372 0.5] Apply Fire Effects Multicast
  (Audio|PlaySoundatLocation (Variables|Audio|GetFireSound) (Transformation|GetActorLocation) "0, 0, 0" 1.0 1.0 0.0 0 0 0 0)
  (Components|Activation|Activate (Variables|Default|GetNiagara) true))

(event Custom|ClearStartFireTimer
  ;[0.15 0 0 0.5] Stop Fire Server
  (Utilities|Time|ClearTimerbyFunctionName 0 "StartFire"))

(event EventDestroyed
  (bind _characterowner (Variables|Default|GetCharacterOwner))
  (Utilities|IsValid _characterowner
    (:Is%20Valid
      (Default|DeleteGunUI _characterowner))))

(event EventTick
  (params (DeltaSeconds :type Float%20%28single-precision%29))
  ;[0 0.15 0.005085 0.5] Recovery
  (CallFunction|RecoilRecovery DeltaSeconds)
  (CallFunction|HeatRecovery DeltaSeconds))

(fn ConstructionScript)

(fn SetCanFire
  (Variables|Global|SetCanFire true)
  (return))

(fn ApplyEffets
  (Transformation|SetRelativeLocation (Variables|Default|GetMesh) "-10.000000,0.000000,0.000000" false false)
  (Components|Activation|Activate (Variables|Default|GetNiagara) true)
  (Audio|PlaySoundatLocation (Variables|Audio|GetFireSound) (Transformation|GetActorLocation) "0, 0, 0" 1.0 1.0 0.0 0 0 0 0)
  (return))

(fn TraceShoot
  (params (ShotSource :type Scene%20Component%20Object%20Reference))
  (bind _returnvalue (Transformation|GetWorldLocation ShotSource))
  (bind _outhit (Collision|LineTraceByChannel _returnvalue (+ _returnvalue (* (Math|Vector|GetForwardVector ShotSource) 50000)) "TraceTypeQuery1" false (Utilities|Array|MakeArray (Variables|Default|GetCharacterOwner)) "None"))
  (return (Utilities|Array|MakeArray _outhit)))

(fn PostShoot
  (if (not (Variables|Reload|GetOverheated))
    (if (Variables|Global|GetAutomatic)
      (Utilities|Time|SetTimerbyFunctionName 0 "StartFire" (Variables|Global|GetFirerate) true)
      (return)
      (else
        (Variables|Global|SetShoted true)
        (return)))))

(fn HeatUp
  (bind _output_get (Variables|Reload|SetHeat (Math|Float|Clamp(Float) (+ (Variables|Reload|GetHeat) (Variables|Reload|GetHearPerShot)) 0.0 (Variables|Reload|GetMaxHeat))))
  (bind _output_get_2 (Variables|Reload|SetOverheated (== _output_get (Variables|Reload|GetMaxHeat))))
  (if _output_get_2
    (CallFunction|StopFire)))

(fn OnRepCharacterOwner)