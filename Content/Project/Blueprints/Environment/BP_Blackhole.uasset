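; Black hole environment actor that emits Geiger-style radiation audio and opens the L_BlackHole level when the player hits its disk collision.
; Construction script drives material size and disk color, and scales the hole and disk collisions from BlackholeSize.
; A self-repeating randomized delay replays the sound, growing louder and more frequent as the player's height difference shrinks relative to squared size, while debug-printing that cubed ratio.
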(event OnComponentHit(DiskCollision)
  (params (HitComponent :type Primitive%20Component%20Object%20Reference) (OtherActor :type Actor%20Object%20Reference) (OtherComp :type Primitive%20Component%20Object%20Reference) (NormalImpulse :type Vector :default "0, 0, 0") (Hit :type Hit%20Result%20Structure%20%28by%20ref%29))
  (if (== OtherActor (Game|Player|GetPlayerPawn 0))
    (Utilities|FlowControl|DoOnce false
      (:Completed
        (Game|OpenLevel(byObjectReference) "/Game/Project/Maps/L_BlackHole.L_BlackHole")))))

(event Custom|PlayGeigerSound
  (bind _returnvalue (Transformation|GetActorLocation))
  (bind _blackhole_size (Variables|Global|GetBlackhole_Size))
  (bind _player_pawn (Variables|Default|GetPlayer%20Pawn))
  (bind _radiationaudiocomponent (Variables|Default|GetRadiationAudioComponent))
  (bind _returnvalue_2 (Transformation|GetActorLocation _player_pawn))
  (bind _returnvalue_3 (Math|Float|Square _blackhole_size))
  (bind _returnvalue_4 (- (.z _returnvalue_2) (.z _returnvalue)))
  (bind _returnvalue_5 (Math|Float|Absolute(Float) _returnvalue_4))
  (bind _returnvalue_6 (/ _returnvalue_5 _returnvalue_3))
  (bind _returnvalue_7 (Math|Float|Power _returnvalue_6 3.0))
  (Audio|Components|Audio|SetVolumeMultiplier _radiationaudiocomponent (/ 1.0 _returnvalue_7) :!class /Script/Engine.AudioComponent)
  (Audio|Components|Audio|Play _radiationaudiocomponent 0.0)
  (Development|PrintString (Utilities|String|ToString(Float) _returnvalue_7))
  (Utilities|FlowControl|Delay (* (Math|Random|RandomFloat) _returnvalue_7))
  (CallFunction|PlayGeigerSound))

(event EventBeginPlay
  (Variables|Default|SetPlayer%20Pawn (Game|Player|GetPlayerPawn 0))
  (CallFunction|PlayGeigerSound))

(event Collision|EventActorBeginOverlap
  (params (OtherActor :type Actor%20Object%20Reference)))

(event EventTick
  (params (DeltaSeconds :type Float%20%28single-precision%29)))

(fn ConstructionScript
  (bind _blackhole_size (Variables|Global|GetBlackhole_Size))
  (Rendering|Material|SetScalarParameterValueonMaterials (Variables|Default|GetBlackhole) "Blackhole_Size" (Variables|Global|GetBlackhole_Size))
  (Rendering|Material|SetVectorParameterValueonMaterials (Variables|Default|GetBlackhole) "Accreation_Disk_Color" (Variables|Details|GetColor))
  (Components|Sphere|SetSphereRadius (Variables|Default|GetHoleCollision) (* (Variables|Global|GetBlackhole_Size) 0.1) true)
  (Components|Box|SetBoxExtent (Variables|Default|GetDiskCollision) (Math|Vector|MakeVector _blackhole_size _blackhole_size (/ _blackhole_size 2e+01)) true))