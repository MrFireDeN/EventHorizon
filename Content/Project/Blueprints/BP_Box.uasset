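; BP_Box is a damageable box actor with a widget health bar that is destroyed when its health runs out.
; On BeginPlay it fills the health on its BPDamageableComponent and hands that component to WBP_HealthBar.
; AnyDamage subtracts directly from the component's health, prints the remainder and destroys the actor at zero or below.
; The Destroyed event spawns the NG_Blood effect at its location; the health OnRep function is empty.
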(event Custom|Apply%20Destruction%20Effects
  (Niagara|SpawnSystematLocation "/Game/Project/FX/NG_Blood.NG_Blood" (Transformation|GetActorLocation)))

(event EventDestroyed
  (CallFunction|ApplyDestructionEffects))

(event EventBeginPlay
  (bind _bp_damageablecomponent (Variables|Default|GetBP_DamageableComponent))
  (bind _output_get (Variables|/Game/Project/Blueprints/BP_DamageableComponent.BP_DamageableComponent_C|SetMaxHealth _bp_damageablecomponent 1e+02))
  (Variables|/Game/Project/Blueprints/BP_DamageableComponent.BP_DamageableComponent_C|SetHealth _bp_damageablecomponent _output_get)
  (bind _aswbp_health_bar (Utilities|Casting|CastToWBP_HealthBar (UserInterface|GetWidget (Variables|Default|GetWidget))))
  (Default|SetDamageableComponent _aswbp_health_bar (Variables|Default|GetBP_DamageableComponent)))

(event Game|Damage|EventAnyDamage
  (params (Damage :type Float%20%28single-precision%29) (DamageType :type Damage%20Type%20Object%20Reference) (InstigatedBy :type Controller%20Object%20Reference) (DamageCauser :type Actor%20Object%20Reference))
  (bind _bp_damageablecomponent (Variables|Default|GetBP_DamageableComponent))
  (bind _output_get (Variables|/Game/Project/Blueprints/BP_DamageableComponent.BP_DamageableComponent_C|SetHealth _bp_damageablecomponent (- (Variables|/Game/Project/Blueprints/BP_DamageableComponent.BP_DamageableComponent_C|GetHealth _bp_damageablecomponent) Damage)))
  (Development|PrintText (Utilities|Text|FormatText "Box: Health left: {Health}" _output_get))
  (if (<= _output_get 0.0)
    (Actor|DestroyActor)))

(fn ConstructionScript)

(fn OnRepHeath)