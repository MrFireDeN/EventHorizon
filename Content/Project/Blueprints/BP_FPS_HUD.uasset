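; BP_FPS_HUD is the first-person player's HUD, managing the on-screen character, gun heat and death widgets.
; It creates the character HUD on BeginPlay and exposes paired Draw and Delete events that add each widget to the viewport or remove it.
; The gun heat widget receives a Gun reference on creation.
; Removal is validity-checked for the gun heat and death widgets, but not the character HUD.
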(event Custom|Draw%20Character%20HUD
  ;[0.15 0.15 0.15 0.5] Player HUD
  (bind _returnvalue (UserInterface|CreateWidget "/Game/Project/UI/WBP_FPS_HUD.WBP_FPS_HUD_C" (Variables|Default|GetPlayerOwner)))
  (UserInterface|Viewport|AddtoViewport _returnvalue 0))

(event Custom|Delete%20Character%20HUD
  ;[0.15 0.15 0.15 0.5] Player HUD
  (Widget|RemovefromParent (stale Custom|Draw%20Character%20HUD _returnvalue)))

(event Custom|Draw%20Gun%20Heat
  (params (Gun :type BP%20Gun%20BASE%20Object%20Reference))
  ;[0.15 0.15 0.15 0.5] Gun Heat
  (bind _returnvalue (UserInterface|CreateWidget "/Game/Project/UI/WPB_GunHeat.WPB_GunHeat_C" (Variables|Default|GetPlayerOwner) Gun))
  (UserInterface|Viewport|AddtoViewport _returnvalue 0))

(event Custom|Delete%20Gun%20Heat
  ;[0.15 0.15 0.15 0.5] Gun Heat
  (Utilities|IsValid (stale Custom|Draw%20Gun%20Heat _returnvalue)
    (:Is%20Valid
      (Widget|RemovefromParent (stale Custom|Draw%20Gun%20Heat _returnvalue)))))

(event Custom|Draw%20Death%20Widget
  (bind _returnvalue (UserInterface|CreateWidget "/Game/Project/UI/WBP_Death.WBP_Death_C" (Variables|Default|GetPlayerOwner)))
  (bind _output_get (Variables|Default|SetDeathWidget _returnvalue))
  (UserInterface|Viewport|AddtoViewport _output_get 0))

(event Custom|Delete%20Death%20Widget
  (bind _deathwidget (Variables|Default|GetDeathWidget))
  (Utilities|IsValid _deathwidget
    (:Is%20Valid
      (Widget|RemovefromParent _deathwidget))))

(event EventBeginPlay
  (CallFunction|DrawCharacterHUD))

(fn ConstructionScript)