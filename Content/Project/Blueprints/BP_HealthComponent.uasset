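; Health component that tracks health and death state for its owner, starting at MaxHealth on BeginPlay.
; TakeDamage ignores non-positive damage or depleted health, doubles head-bone hits, fires OnTakeDamage, then subtracts health and returns IsDead and remaining health.
; Health and MaxHealth use RepNotify: Health changes broadcast OnHealthChanged, and MaxHealth changes reset Health to the new maximum.
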(event EventBeginPlay
  (Variables|Default|SetHealth (Variables|Default|GetMaxHealth)))

(fn OnRepHealth
  (Default|CallOnHealthChanged (Variables|Default|GetHealth) (Variables|Default|GetMaxHealth)))

(fn TakeDamage
  (params (Damage :type Float%20%28double-precision%29) (Bone :type Name))
  (bind _returnvalue (== Bone "head"))
  (bind _returnvalue_2 (* Damage 2.0))
  (bind _returnvalue_3 (select _returnvalue _returnvalue_2 Damage))
  ;[0.15 0.15 0.15 0.5] Take Damage
  ;;[0.15 0.15 0.15 0.5] Damage and Health Check
  (if (and (> Damage 0.0) (> (Variables|Default|GetHealth) 0.0))
    ;;[0.15 0.15 0.15 0.5] Set New Health
    (Default|CallOnTakeDamage _returnvalue_3)
    (bind _output_get (Variables|Default|SetHealth (- (Variables|Default|GetHealth) _returnvalue_3)))
    (bind _output_get_2 (Variables|Default|SetIsDead (<= _output_get 0.0)))
    (return _output_get_2 _output_get)))

(fn OnRepMaxHealth
  (Variables|Default|SetHealth (Variables|Default|GetMaxHealth)))