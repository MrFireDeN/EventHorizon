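; BP_FPS_Character is a first-person shooter character with a swappable gun, walk speed setup and health.
; The gun lives in a child actor component, and ChangeGun swaps its class and caches it as CurrentGun.
; Point damage doubles on head hits, spawns blood and sound at the impact, and destroys the character at zero health.
; ChangeView hides and de-collides the body mesh for player-controlled characters, otherwise hiding the gun component.
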(event Custom|ChangeGun
  (params (GunClass :type BP%20Gun%20BASE%20Class%20Reference))
  (bind _bp_gun (Variables|Default|GetBP_Gun))
  (ChildActorComponent|SetChildActorClass _bp_gun GunClass)
  (bind _asbp_gun_base (Utilities|Casting|CastToBP_Gun_BASE (Variables|/Script/Engine.ChildActorComponent|GetChildActor _bp_gun)))
  (Variables|Default|SetCurrentGun _asbp_gun_base))

(event EventBeginPlay
  (Variables|/Script/Engine.CharacterMovementComponent|SetMaxWalkSpeed (Variables|Character|GetCharacterMovement) (Variables|Movement|GetWalkSpeed))
  (bind _asbp_gun_base (Utilities|Casting|CastToBP_Gun_BASE (Variables|/Script/Engine.ChildActorComponent|GetChildActor (Variables|Default|GetBP_Gun))))
  (Variables|Default|SetCurrentGun _asbp_gun_base)
  (CallFunction|ChangeView))

(event Game|Damage|EventPointDamage
  (params (Damage :type Float%20%28single-precision%29) (DamageType :type Damage%20Type%20Object%20Reference) (HitLocation :type Vector :default "0, 0, 0") (HitNormal :type Vector :default "0, 0, 0") (HitComponent :type Primitive%20Component%20Object%20Reference) (BoneName :type Name :default "None") (ShotFromDirection :type Vector :default "0, 0, 0") (InstigatedBy :type Controller%20Object%20Reference) (DamageCauser :type Actor%20Object%20Reference) (HitInfo :type Hit%20Result%20Structure%20%28by%20ref%29))
  (Variables|Damage|SetDamage Damage)
  (Variables|Damage|SetHit%20Location HitLocation)
  (Variables|Damage|SetHit%20Normal HitNormal)
  (bind _output_get (Variables|Damage|SetBone%20Name BoneName))
  (Variables|General|SetHealth (- (Variables|General|GetHealth) (select (== _output_get "head") (* (Variables|Damage|GetDamage) 2.0) (Variables|Damage|GetDamage))))
  (Niagara|SpawnSystematLocation "/Game/Project/FX/NG_Blood.NG_Blood" (Variables|Damage|GetHit%20Location) (Math|Conversions|RotationFromXVector (Variables|Damage|GetHit%20Normal)))
  (Audio|PlaySoundatLocation "/Engine/EditorSounds/GamePreview/EndPlayInEditor.EndPlayInEditor" (Variables|Damage|GetHit%20Location) "0, 0, 0" 1.0 1.0 0.0 0 0 0 0)
  (if (<= (Variables|General|GetHealth) 0.0)
    (Actor|DestroyActor)))

(fn ConstructionScript)

(fn ChangeView
  (bind _mesh (Variables|Character|GetMesh))
  (if (Pawn|IsPlayerControlled)
    (Rendering|SetVisibility _mesh false true)
    (Collision|SetCollisionEnabled _mesh "NoCollision")
    (else
      (Rendering|SetVisibility (Variables|Default|GetBP_Gun) false false)))
  (return))